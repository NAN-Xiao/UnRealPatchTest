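; Manager actor for Jiffycrew post-process line rendering: silhouette, crease, suggestive contour and highlight lines.
; Construction creates a dynamic material on its PostProcess at 200% screen percentage.
; BeginPlay and every Tick push line settings to the material, scaling widths by screen percentage, and set blend weight from ShowLines.
; EnableLinesOnActor turns on an actor's custom depth; DisableLinesOnActor also sets it true, on the manager itself.
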(event `self.ReceiveBeginPlay`
  (`self.UpdateLineParameters` (* (`.ScreenPercentage` (break `PostProcessSettings` (`PostProcessComponent.Settings` (`self.PostProcess`)))) 0.01) :!label _label)
  (set `PostProcessComponent.BlendWeight` (`KismetMathLibrary.Conv_BoolToDouble` (`self.Show lines`)) (`self.PostProcess`)))

(event `self.ReceiveTick`
  (params (DeltaSeconds :type "Float (single-precision)"))
  (goto _label))

(fn `DisableLinesOnActor`
  (`PrimitiveComponent.SetRenderCustomDepth` (`self.GetComponentByClass` "/Script/Engine.MeshComponent") true))

(fn `EnableLinesOnActor`
  (params (actor :type "Actor Object Reference"))
  (`PrimitiveComponent.SetRenderCustomDepth` (`self.GetComponentByClass` actor "/Script/Engine.MeshComponent") true))

(fn `UpdateLineParameters`
  (params (WidthMultiplier :type "Float (double-precision)"))
  (locals (NewLocalVar_0 :type Boolean))
  (`|ExecutionSequence`
    (:`then_1`
      ;[1 1 1] Global
      (`MaterialInstanceDynamic.SetScalarParameterValue` (`self.PPMaterial`) "AugmentSceneColor" (`KismetMathLibrary.Conv_BoolToDouble` (`self.AugmentSceneRendering`)))
      (`MaterialInstanceDynamic.SetScalarParameterValue` (`self.PPMaterial`) "MultiplyLineColor" (`KismetMathLibrary.Conv_BoolToDouble` (`self.MultiplyLineColor`)))
      (`MaterialInstanceDynamic.SetScalarParameterValue` (`self.PPMaterial`) "UseCustomDepth" (`KismetMathLibrary.Conv_BoolToDouble` (`self.UseCustomDepth`)))
      (`MaterialInstanceDynamic.SetScalarParameterValue` (`self.PPMaterial`) "UseDepthAdaptation" (`KismetMathLibrary.Conv_BoolToDouble` (`self.UseDepthAdaptation`)))
      (`MaterialInstanceDynamic.SetScalarParameterValue` (`self.PPMaterial`) "BaseDepth" (`self.BaseDepthForDepthAdaptation`))
      (`MaterialInstanceDynamic.SetVectorParameterValue` (`self.PPMaterial`) "BackgroundColor" (`KismetMathLibrary.Conv_ColorToLinearColor` (`self.BackgroundColor`))))
    (:`then_2`
      ;[1 1 1] Line Enable
      (`MaterialInstanceDynamic.SetScalarParameterValue` (`self.PPMaterial`) "SilhouetteLineEnable" (`KismetMathLibrary.Conv_BoolToDouble` (`self.SilhouetteLineEnable`)))
      (`MaterialInstanceDynamic.SetScalarParameterValue` (`self.PPMaterial`) "CreaseLineEnable" (`KismetMathLibrary.Conv_BoolToDouble` (`self.CreaseLineEnable`)))
      (`MaterialInstanceDynamic.SetScalarParameterValue` (`self.PPMaterial`) "SuggestiveContourLineEnable" (`KismetMathLibrary.Conv_BoolToDouble` (`self.SuggestiveContourLineEnable`)))
      (`MaterialInstanceDynamic.SetScalarParameterValue` (`self.PPMaterial`) "SuggestiveHighlightLineEnable" (`KismetMathLibrary.Conv_BoolToDouble` (`self.SuggestiveHighlightLineEnable`))))
    (:`then_3`
      ;[1 1 1] Line Color
      (`MaterialInstanceDynamic.SetVectorParameterValue` (`self.PPMaterial`) "Silhouette Line Color" (`KismetMathLibrary.Conv_ColorToLinearColor` (`self.SilhouetteLineColor`)))
      (`MaterialInstanceDynamic.SetVectorParameterValue` (`self.PPMaterial`) "Crease Line Color" (`KismetMathLibrary.Conv_ColorToLinearColor` (`self.CreaseLineColor`)))
      (`MaterialInstanceDynamic.SetVectorParameterValue` (`self.PPMaterial`) "Suggestive Contour Line Color" (`KismetMathLibrary.Conv_ColorToLinearColor` (`self.SuggestiveContourLineColor`)))
      (`MaterialInstanceDynamic.SetVectorParameterValue` (`self.PPMaterial`) "Suggestive Highlight Line Color" (`KismetMathLibrary.Conv_ColorToLinearColor` (`self.SuggestiveHighlightLineColor`))))
    (:`then_4`
      ;[1 1 1] Line Width
      (`MaterialInstanceDynamic.SetScalarParameterValue` (`self.PPMaterial`) "SilhouetteLineWidth" (* (`self.SilhouetteLineWidth`) (`local.WidthMultiplier`)))
      (`MaterialInstanceDynamic.SetScalarParameterValue` (`self.PPMaterial`) "CreaseLineWidth" (* (`self.CreaseLineWidth`) (`local.WidthMultiplier`)))
      (`MaterialInstanceDynamic.SetScalarParameterValue` (`self.PPMaterial`) "SuggestiveContourLineWidth" (* (`self.SuggestiveContourLineWidth`) (`local.WidthMultiplier`)))
      (`MaterialInstanceDynamic.SetScalarParameterValue` (`self.PPMaterial`) "SuggestiveHighlightLineWidth" (* (`self.SuggestiveHighlightLineWidth`) (`local.WidthMultiplier`))))
    (:`then_5`
      ;[1 1 1] Line Threshold
      (`MaterialInstanceDynamic.SetScalarParameterValue` (`self.PPMaterial`) "SilhouetteLineThreshold" (`self.SilhouetteLineThreshold`))
      (`MaterialInstanceDynamic.SetScalarParameterValue` (`self.PPMaterial`) "CreaseLineThreshold" (`self.CreaseLineThreshold`))
      (`MaterialInstanceDynamic.SetScalarParameterValue` (`self.PPMaterial`) "SuggestiveContourLineThreshold" (`self.SuggestiveContourLineThreshold`))
      (`MaterialInstanceDynamic.SetScalarParameterValue` (`self.PPMaterial`) "SuggestiveHighlightLineThreshold" (`self.SuggestiveHighlightLineThreshold`)))))

(fn `UserConstructionScript`
  (bind _returnvalue (`KismetMaterialLibrary.CreateDynamicMaterialInstance` "/Game/JiffycrewPPLine/Materials/PP_JiffycrewPPLine.PP_JiffycrewPPLine"))
  (set `self.ppMaterial` _returnvalue)
  (set `PostProcessComponent.Settings` (make `PostProcessSettings` :`AmbientOcclusionIntensity` 0.0 :`ScreenPercentage` 200.0 :`WeightedBlendables` (make `WeightedBlendables` (`|MakeArray` (make `WeightedBlendable` (`KismetMathLibrary.Conv_BoolToDouble` (`self.Show lines`)) (`self.PPMaterial`))))) (`self.PostProcess`))
  (`self.UpdateLineParameters` 1.0))